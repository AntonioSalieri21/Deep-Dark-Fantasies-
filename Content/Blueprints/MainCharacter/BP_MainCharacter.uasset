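; Main character Blueprint that moves along the world X axis, snapping its yaw to face right or left, with forgiving jump timing.
; Tick keeps a coyote-time grounded flag alive briefly after leaving the ground.
; Pressing Jump opens a countdown buffer, during which Tick calls Jump whenever that flag is set, so early and late presses still register.
; Debug strings print the buffer state.
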(event `self.ReceiveBeginPlay`
  (set `self.DelayBeforeLand` (`self.MaxDelayBeforeLand`))
  (set `self.DelayAfterFall` (`self.MaxDelayAfterFall`)))

(event `self.ReceiveTick`
  (params (DeltaSeconds :type "Float (single-precision)"))
  (`|ExecutionSequence`
    (:`then_0`
      (`self.K2_SetActorRotation` (`KismetMathLibrary.MakeRotator` 0.0 0.0 (`self.CurrentRotation`))))
    (:`then_1`
      (if (`NavMovementComponent.IsMovingOnGround` (`self.CharacterMovement`))
        (set `self.WasGrounded` true)
        (set `self.DelayAfterFall` (`self.MaxDelayAfterFall`))
        (else
          (bind _output_get (set `self.DelayAfterFall` (- (`self.DelayAfterFall`) DeltaSeconds)))
          (if (<= _output_get 0.0)
            (set `self.WasGrounded` false)))))
    (:`then_2`
      (if (`self.PressedJump`)
        (bind _output_get_2 (set `self.DelayBeforeLand` (- (`self.DelayBeforeLand`) DeltaSeconds)))
        (if (>= _output_get_2 0.0)
          (`KismetSystemLibrary.PrintString` "True")
          (if (`self.WasGrounded`)
            (`self.Jump`))
          (else
            (set `self.PressedJump` false)
            (set `self.DelayBeforeLand` (`self.MaxDelayBeforeLand`))
            (`KismetSystemLibrary.PrintString` "False")))))
    (:`then_3`)))

(event `InputAxis|Move_Right`
  (params (AxisValue :type "Float (single-precision)"))
  (if (> AxisValue 0.0)
    (`self.AddMovementInput` (1.0 0.0 0.0) AxisValue)
    (`/Engine/EditorBlueprintResources/StandardMacros.CompareFloat` AxisValue :!label _label
      (:`>`
        (set `self.CurrentRotation` 0.0))
      (:`<`
        (set `self.CurrentRotation` 180.0)))
    (elif (< AxisValue 0.0)
      (`self.AddMovementInput` (1.0 0.0 0.0) AxisValue)
      (goto _label))))

(event `InputAction|Jump`
  (params (Key :type "Key Structure"))
  (:`Pressed`
    (set `self.PressedJump` true)))

(fn `UserConstructionScript`)